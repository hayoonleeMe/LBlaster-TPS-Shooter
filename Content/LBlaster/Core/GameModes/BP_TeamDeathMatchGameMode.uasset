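; BP_TeamDeathMatchGameMode is the team deathmatch game mode Blueprint, which customizes player start selection.
; Its FindPlayerStart override calls FindPlayerStartTDM for the player and uses that result when valid.
; Otherwise it falls back to the parent's FindPlayerStart with the player and incoming name.
; BeginPlay and Tick are disabled stubs, and the construction script only calls its parent.
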(fn `FindPlayerStart`
  (params (Player :type "Controller Object Reference") (IncomingName :type String))
  (returns (ReturnValue :type "Actor Object Reference"))
  (bind _returnvalue (`self.FindPlayerStartTDM` Player))
  (`/Engine/EditorBlueprintResources/StandardMacros.IsValid` _returnvalue
    (:`Is Valid`
      (return _returnvalue))
    (:`Is Not Valid`
      (bind _returnvalue_2 (`parent.FindPlayerStart` (`local.Player`) (`local.IncomingName`)))
      (return _returnvalue_2))))

(fn `UserConstructionScript`
  (`parent.UserConstructionScript`))